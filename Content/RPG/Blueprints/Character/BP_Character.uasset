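; BP_Character is a player character with movement, look, weapon controls, aiming and damage feedback.
; Input drives movement and look directly, and forwards fire, reload and slot selection on number keys to a Weapon component.
; Aiming plays or reverses a timeline that changes camera FOV, while AimServer stores the Aiming state.
; Damage prints its amount, then, for player-controlled characters, DamageClient triggers a camera shake and BP_HUD damage feedback.
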(event Custom|DamageClient
  (bind _asplayer_controller (Utilities|Casting|CastToPlayerController (Pawn|GetController)))
  (CameraShakes|StartCameraShake (Variables|/Script/Engine.PlayerController|GetPlayerCameraManager _asplayer_controller) "/Game/RPG/VFX/CameraShake/BP_DamageCameraShake.BP_DamageCameraShake_C" 1.0 "CameraLocal" "0, 0, 0")
  (Default|Damage (.AsBP%20HUD (Utilities|Casting|CastToBP_HUD (HUD|GetHUD _asplayer_controller)))))

(event Custom|AimServer
  (params (Aiming :type Boolean))
  (Variables|Default|SetAiming Aiming))

(event Game|Damage|EventAnyDamage
  (params (Damage :type Float%20%28single-precision%29) (DamageType :type Damage%20Type%20Object%20Reference) (InstigatedBy :type Controller%20Object%20Reference) (DamageCauser :type Actor%20Object%20Reference))
  (Development|PrintString (Utilities|String|ToString(Float) Damage) true true "(R=1.000000,G=0.000000,B=0.067612,A=1.000000)" 1.0)
  (Utilities|Casting|CastToPlayerController (Pawn|GetController))
  (CallFunction|DamageClient))

(event Input|ActionEvents|InputActionFire
  (params (Key :type Key%20Structure :default "None"))
  (:Pressed
    (Class|WeaponComponent|StartFire (Variables|Default|GetWeapon)))
  (:Released
    (Class|WeaponComponent|StopFire (Variables|Default|GetWeapon))))

(event Input|ActionEvents|InputActionReload
  (params (Key :type Key%20Structure :default "None"))
  (:Pressed
    (Class|WeaponComponent|Reload (Variables|Default|GetWeapon))))

(event Input|ActionEvents|InputActionAim
  (params (Key :type Key%20Structure :default "None"))
  (:Pressed
    (CallFunction|AimServer true)
    (bind _fieldofview (Timeline|AimTimeline Play)
      (:Update
        (Camera|SetFieldOfView (Variables|Default|GetCamera) _fieldofview))))
  (:Released
    (CallFunction|AimServer false)
    (Timeline|AimTimeline Reverse)))

(event Input|AxisEvents|InputAxisMoveForward
  (params (AxisValue :type Float%20%28single-precision%29))
  (Pawn|Input|AddMovementInput (Transformation|GetActorForwardVector) AxisValue false))

(event Input|AxisEvents|InputAxisMoveRight
  (params (AxisValue :type Float%20%28single-precision%29))
  (Pawn|Input|AddMovementInput (Transformation|GetActorRightVector) AxisValue false))

(event Input|AxisEvents|InputAxisLookUp
  (params (AxisValue :type Float%20%28single-precision%29))
  (Pawn|Input|AddControllerPitchInput AxisValue))

(event Input|AxisEvents|InputAxisTurn
  (params (AxisValue :type Float%20%28single-precision%29))
  (Pawn|Input|AddControllerYawInput AxisValue))

(event Input|KeyboardEvents|1
  (params (Key :type Key%20Structure :default "None"))
  (:Pressed
    (Class|WeaponComponent|SelectWeapon (Variables|Default|GetWeapon) 1)))

(event Input|KeyboardEvents|2
  (params (Key :type Key%20Structure :default "None"))
  (:Pressed
    (Class|WeaponComponent|SelectWeapon (Variables|Default|GetWeapon) 2)))

(event Input|KeyboardEvents|3
  (params (Key :type Key%20Structure :default "None"))
  (:Pressed
    (Class|WeaponComponent|SelectWeapon (Variables|Default|GetWeapon) 3)))

(event Input|KeyboardEvents|4
  (params (Key :type Key%20Structure :default "None"))
  (:Pressed
    (Class|WeaponComponent|SelectWeapon (Variables|Default|GetWeapon) 4)))

(fn ConstructionScript)